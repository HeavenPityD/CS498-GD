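; BP_TunnelSpawner builds a chain of BP_Tunnel segments for a tunnel level.
; On BeginPlay it clears existing tunnels and health packs, then spawns an initial run starting at the player pawn.
; Each new segment attaches at the newest tunnel's SpawnPoint, gets a spawner back-reference and randomizes its wall.
; Each spawn also independently rolls a small chance of a randomly offset Health_Pack and Enemy.
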(event EventBeginPlay
  (CallFunction|SpawnInitialTunnels))

(fn ConstructionScript)

(fn SpawnTunnel
  (params (SpawnLocation :type Vector))
  (bind _returnvalue (Game|SpawnActorfromClass "/Game/InfiniteMatrix/Blueprints/BP_Tunnel.BP_Tunnel_C" (Math|Transform|MakeTransform SpawnLocation "0, 0, 0" "1,1,1") "Undefined" 0 0))
  (if (== (Math|Random|RandomIntegerinRange 0 7) 0)
    (Game|SpawnActorfromClass "/Game/InfiniteMatrix/Blueprints/Health_Pack.Health_Pack_C" (Math|Transform|MakeTransform (+ SpawnLocation (Math|Vector|MakeVector (Math|Random|RandomFloatinRange 5e+02 1.5e+03) (Math|Random|RandomFloatinRange 0.0 2.5e+02) (Math|Random|RandomFloatinRange 0.0 2.5e+02))) "0, 0, 0" "1,1,1") "Undefined" 0 0))
  (bind _output_get (Variables|Default|SetNewestTunnel _returnvalue))
  (Variables|/Game/InfiniteMatrix/Blueprints/BP_Tunnel.BP_Tunnel_C|SetTunnelSpawner _output_get self)
  (Default|RandomizeWall _output_get)
  (if (== (Math|Random|RandomIntegerinRange 0 7) 0)
    (Game|SpawnActorfromClass "/Game/InfiniteMatrix/Blueprints/enemy.enemy_C" (Math|Transform|MakeTransform (+ SpawnLocation (Math|Vector|MakeVector (Math|Random|RandomFloatinRange 5e+02 1.5e+03) (Math|Random|RandomFloatinRange 0.0 2.5e+02) (Math|Random|RandomFloatinRange 0.0 2.5e+02))) "0, 0, 0" "1,1,1") "Undefined" 0 0)))

(fn SpawnTunnelatSpawnPoint
  (CallFunction|SpawnTunnel (Transformation|GetWorldLocation (Variables|/Game/InfiniteMatrix/Blueprints/BP_Tunnel.BP_Tunnel_C|GetSpawnPoint (Variables|Default|GetNewestTunnel)))))

(fn SpawnInitialTunnels
  (Utilities|FlowControl|Sequence
    (:then_0
      (bind _outactors (Actor|GetAllActorsOfClass "/Game/InfiniteMatrix/Blueprints/BP_Tunnel.BP_Tunnel_C"))
      (for _array_element _outactors
        (Actor|DestroyActor _array_element)
        (bind _outactors_2 (Actor|GetAllActorsOfClass "/Game/InfiniteMatrix/Blueprints/Health_Pack.Health_Pack_C"))
        (for _array_element_2 _outactors_2
          (Actor|DestroyActor _array_element_2))))
    (:then_1
      (for _index (range 0 2)
        (Utilities|IsValid (Variables|Default|GetNewestTunnel)
          (:Is%20Valid
            (CallFunction|SpawnTunnelatSpawnPoint))
          (:Is%20Not%20Valid
            (CallFunction|SpawnTunnel (Transformation|GetActorLocation (Game|Player|GetPlayerPawn 0)))))))))